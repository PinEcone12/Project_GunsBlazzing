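; BP_Health_Comp is a health component for the weapon system, handling damage, full restore and health recovery on its owner.
; Damage lowers health, and reaching zero fires a resettable DoOnce that clears the recovery timer.
; Recovery clamps its target to max health and binds a lerp step toward it to a timer, though that timer is set with zero time and no looping.
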(event `self.ReceiveBeginPlay`
  (set `self.Charecter` (`self.GetOwner`)))

(event `ResetDeathEvent`
  (goto _label :!via `Reset`))

(event `Damage`
  (params (Damage :type "Float (double-precision)") (DamageCauser :type "Actor Object Reference"))
  (bind _health (`self.Health`))
  (set `self.Health` (`KismetMathLibrary.FClamp` (- _health Damage) 0.0 _health))
  (if (== (`self.Health`) 0.0)
    (`/Engine/EditorBlueprintResources/StandardMacros.DoOnce` false :!label _label
      (:`Completed`
        (`KismetSystemLibrary.K2_ClearAndInvalidateTimerHandle` (`self.HealthRestore_Timer`))))))

(event `FullHealthRestore`
  (set `self.Health` (`self.MaxHealth`)))

(event `StartHealthRecovery`
  ;[1 1 1] Recovery Health Timer
  (if (>= (`self.HealthRecoveryTime`) 0.0)
    (set `self.HealthRecoveryValue` (select `bool` (== (`self.HealthRecoveryValue`) 0.0) :`false` (`KismetMathLibrary.FClamp` (`self.HealthRecoveryValue`) 0.0 (`self.MaxHealth`)) :`true` (`self.MaxHealth`)))
    (if (> (`self.HealthRecoveryValue`) (`self.Health`))
      (set `self.CurrentHealth` (`self.Health`))
      (set `self.CurrentTime` 0.0)
      (bind _returnvalue (`KismetSystemLibrary.K2_SetTimerDelegate` (delegate `HealthRecovery`)))
      (set `self.HealthRestore_Timer` _returnvalue))))

(event `HealthRecovery`
  (bind _healthrecoverytime (`self.HealthRecoveryTime`))
  (bind _healthrecoverytime_2 (`self.HealthRecoveryTime`))
  ;[1 1 1] Recovery Health Timer
  (set `self.Health` (`KismetMathLibrary.Lerp` (`self.CurrentHealth`) (`self.HealthRecoveryValue`) (/ (`self.CurrentTime`) (`KismetMathLibrary.FClamp` _healthrecoverytime 0.0 _healthrecoverytime))))
  (bind _output_get (set `self.CurrentTime` (+ (`self.CurrentTime`) 1.0)))
  (if (> _output_get (`KismetMathLibrary.FClamp` _healthrecoverytime_2 1.0 _healthrecoverytime_2))
    (set `self.Health` (`self.HealthRecoveryValue`))
    (`KismetSystemLibrary.K2_ClearAndInvalidateTimerHandle` (`self.HealthRestore_Timer`))))