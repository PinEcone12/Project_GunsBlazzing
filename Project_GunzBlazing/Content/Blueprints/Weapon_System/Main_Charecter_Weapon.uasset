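; Main_Charecter_Weapon is a weapon-system Blueprint with a single helper, MainFunction, that tracks named value modifiers in a map.
; Adding stores a new key's value and returns base plus that value, with no return wired for existing keys.
; Removing deletes the key and returns the stored value minus base (not base minus stored), or zero if absent.
; The event graph holds only disabled BeginPlay and Tick stubs.
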(fn `MainFunction`
  (params (BaseValue :type "Float (double-precision)") (AddValue :type "Float (double-precision)") (MapType :type "Map of String to Float (double-precision)") (Remove :type Boolean) (TypeName :type String))
  (returns (FinalValue :type "Float (double-precision)") (Finalmap :type "Map of String to Float (double-precision)"))
  (bind (_value _returnvalue) (`BlueprintMapLibrary.Map_Find` MapType TypeName))
  (if _returnvalue
    (if Remove
      (set `self.FinalValueLocal` (- _value BaseValue))
      (`BlueprintMapLibrary.Map_Remove` MapType TypeName)
      (return (`self.FinalValueLocal`) MapType))
    (elif Remove
      (return 0.0 MapType)
      (else
        (`BlueprintMapLibrary.Map_Add` MapType TypeName AddValue)
        (return (+ BaseValue AddValue) MapType)))))