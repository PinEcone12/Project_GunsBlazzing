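; Weapon storage Blueprint that holds weapon data in name-keyed maps and equips it onto a passed-in weapon component.
; AddWeapon sets the component from WeaponList, while ChangeWeapon sets it from AvailableWeapons, both printing a placeholder "Hello" when the name is missing.
; SaveWeapon writes the component's current weapon struct into AvailableWeapons, which other functions list by key or remove from.
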(fn `AddWeapon`
  (params (WeaponName :type String) (WeaponComponent :type "/Game/Blueprints/Weapon_System/BP_MainWeapon Object Reference"))
  (bind (_value _returnvalue) (`BlueprintMapLibrary.Map_Find` (`self.WeaponList`) WeaponName))
  (if _returnvalue
    (`/Game/Blueprints/Weapon_System/BP_MainWeapon.SetWeapon` WeaponComponent _value)
    (else
      (`KismetSystemLibrary.PrintString` "Hello"))))

(fn `ChangeWeapon`
  (params (weaponName :type String) (weaponComponent :type "/Game/Blueprints/Weapon_System/BP_MainWeapon Object Reference"))
  (bind (_value _returnvalue) (`BlueprintMapLibrary.Map_Find` (`self.AvailableWeapons`) weaponName))
  (if _returnvalue
    (`/Game/Blueprints/Weapon_System/BP_MainWeapon.SetWeapon` weaponComponent _value)
    (else
      (`KismetSystemLibrary.PrintString` "Hello"))))

(fn `GetAvailableWeapons`
  (returns (AvailableWeapons :type "Array of String"))
  (bind _keys (`BlueprintMapLibrary.Map_Keys` (`self.AvailableWeapons`)))
  (return _keys))

(fn `RemoveWeapon`
  (params (`Weapon Name` :type String))
  (`BlueprintMapLibrary.Map_Remove` (`self.AvailableWeapons`) `Weapon Name`))

(fn `SaveWeapon`
  (params (WeaponComponent :type "/Game/Blueprints/Weapon_System/BP_MainWeapon Object Reference"))
  (`BlueprintMapLibrary.Map_Add` (`self.AvailableWeapons`) (`/Game/Blueprints/Weapon_System/BP_MainWeapon.weaponName` WeaponComponent) (`/Game/Blueprints/Weapon_System/BP_MainWeapon.WeaponStruct` WeaponComponent)))